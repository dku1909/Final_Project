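; A locked door that the third-person character opens with the Interact input when holding the second key (Haskey2).
; Overlapping its box enables input, caches the character and opens a Gate node; leaving reverses the input and gate.
; With the key, a FlipFlop's A output plays a timeline that lerps mesh yaw from closed to open; B is unwired.
; Without it, "No Key!" prints on screen.
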(event OnComponentBeginOverlap(Box)
  (params (OverlappedComponent :type Primitive%20Component%20Object%20Reference) (OtherActor :type Actor%20Object%20Reference) (OtherComp :type Primitive%20Component%20Object%20Reference) (OtherBodyIndex :type Integer) (bFromSweep :type Boolean) (SweepResult :type Hit%20Result%20Structure%20%28by%20ref%29))
  (bind _asthird_person_character (Utilities|Casting|CastToThirdPersonCharacter OtherActor))
  (Input|EnableInput (Game|GetPlayerController 0))
  (Utilities|FlowControl|Gate true) ; enters at Open
)

(event OnComponentEndOverlap(Box)
  (params (OverlappedComponent :type Primitive%20Component%20Object%20Reference) (OtherActor :type Actor%20Object%20Reference) (OtherComp :type Primitive%20Component%20Object%20Reference) (OtherBodyIndex :type Integer))
  (Utilities|Casting|CastToThirdPersonCharacter OtherActor)
  (Input|DisableInput (Game|GetPlayerController 0))
  (Utilities|FlowControl|Gate true) ; enters at Close
)

(event Input|ActionEvents|InputActionInteract
  (params (Key :type Key%20Structure :default "None"))
  (:Pressed
    (if (Variables|/Game/ThirdPersonBP/Blueprints/ThirdPersonCharacter.ThirdPersonCharacter_C|GetHaskey2? (stale OnComponentBeginOverlap(Box) _asthird_person_character))
      (Utilities|FlowControl|Gate true
        (:Exit
          (Utilities|FlowControl|FlipFlop
            (:A
              (bind _open_close (Timeline|Timeline_0 Play)
                (:Update
                  (Transformation|SetRelativeRotation (Variables|Default|GetStaticMesh) (Math|Rotator|MakeRotator 0.0 0.0 (Math|Float|Lerp (Variables|Default|GetClosed%20Angle) (Variables|Default|GetOpen%20Angle) _open_close)) false false)))))))
      (else
        (Development|PrintString "No Key!" true true "(R=1.000000,G=0.156221,B=0.162853,A=1.000000)" 5.0)))))

(fn ConstructionScript)