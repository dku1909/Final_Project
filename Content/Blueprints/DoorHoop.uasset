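; DoorHoop is a locked door that swings open when the player character interacts with it while holding the hoop key.
; A box trigger shows the interact prompt, enables input and opens a gate while the character is inside.
; With the key, Interact passes the gate and a FlipFlop to play a timeline that rotates the mesh's yaw; no closing branch is wired.
; Without it, a lock sound plays and a text widget appears briefly.
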(event OnComponentBeginOverlap(Box)
  (params (OverlappedComponent :type Primitive%20Component%20Object%20Reference) (OtherActor :type Actor%20Object%20Reference) (OtherComp :type Primitive%20Component%20Object%20Reference) (OtherBodyIndex :type Integer) (bFromSweep :type Boolean) (SweepResult :type Hit%20Result%20Structure%20%28by%20ref%29))
  (bind _asthird_person_character (Utilities|Casting|CastToThirdPersonCharacter OtherActor))
  (bind _returnvalue (UserInterface|CreateWidget "/Game/Blueprints/UseEtointeract.UseEtointeract_C"))
  (UserInterface|Viewport|AddtoViewport _returnvalue 0)
  (Input|EnableInput (Game|GetPlayerController 0))
  (Utilities|FlowControl|Gate true) ; enters at Open
)

(event OnComponentEndOverlap(Box)
  (params (OverlappedComponent :type Primitive%20Component%20Object%20Reference) (OtherActor :type Actor%20Object%20Reference) (OtherComp :type Primitive%20Component%20Object%20Reference) (OtherBodyIndex :type Integer))
  (Utilities|Casting|CastToThirdPersonCharacter OtherActor)
  (Widget|RemovefromParent (stale OnComponentBeginOverlap(Box) _returnvalue))
  (Input|DisableInput (Game|GetPlayerController 0))
  (Utilities|FlowControl|Gate true) ; enters at Close
)

(event Input|ActionEvents|InputActionInteract
  (params (Key :type Key%20Structure :default "None"))
  (:Pressed
    (Variables|/Game/Blueprints/UseEtointeract.UseEtointeract_C|SetIs%20Pressed? (stale OnComponentBeginOverlap(Box) _returnvalue) true)
    (Utilities|FlowControl|Delay 0.2)
    (Variables|/Game/Blueprints/UseEtointeract.UseEtointeract_C|SetIs%20Pressed? (stale OnComponentBeginOverlap(Box) _returnvalue) false)
    (if (Variables|/Game/ThirdPersonBP/Blueprints/ThirdPersonCharacter.ThirdPersonCharacter_C|GetHas%20keyhoop? (stale OnComponentBeginOverlap(Box) _asthird_person_character))
      (Utilities|FlowControl|Gate true
        (:Exit
          (Utilities|FlowControl|FlipFlop
            (:A
              (bind _open_close (Timeline|Timeline_0 Play)
                (:Update
                  (Transformation|SetRelativeRotation (Variables|Default|GetStaticMesh) (Math|Rotator|MakeRotator 0.0 0.0 (Math|Float|Lerp (Variables|Default|GetClosed%20a) (Variables|Default|GetOpen%20a) _open_close)) false false)))))))
      (else
        (Audio|PlaySoundatLocation "/Game/Blueprints/Door_Lock_Sound_Effect.Door_Lock_Sound_Effect" "0, 0, 0" "0, 0, 0" 1.0 1.0 0.0 0 0 0)
        (bind _returnvalue (UserInterface|CreateWidget "/Game/Blueprints/TextResponse.TextResponse_C"))
        (UserInterface|Viewport|AddtoViewport _returnvalue 0)
        (Utilities|FlowControl|Delay 3.0)
        (Widget|RemovefromParent _returnvalue)))))

(fn ConstructionScript)