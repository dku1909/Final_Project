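; DoorButton1 is a button-operated door that the player toggles open and closed with the Interact input.
; Overlapping InteractionBox shows a prompt widget, enables input and opens a gate for the press.
; Each press plays a button-push timeline, then a FlipFlop plays or reverses the door's yaw timeline.
; Leaving the box only removes the prompt; the DisableInput and gate-close nodes are unconnected, so the button stays usable.
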(event OnComponentBeginOverlap(interactionbox)
  (params (OverlappedComponent :type Primitive%20Component%20Object%20Reference) (OtherActor :type Actor%20Object%20Reference) (OtherComp :type Primitive%20Component%20Object%20Reference) (OtherBodyIndex :type Integer) (bFromSweep :type Boolean) (SweepResult :type Hit%20Result%20Structure%20%28by%20ref%29))
  (Utilities|Casting|CastToThirdPersonCharacter OtherActor)
  (bind _returnvalue (UserInterface|CreateWidget "/Game/Blueprints/UseEtointeract.UseEtointeract_C"))
  (UserInterface|Viewport|AddtoViewport _returnvalue 0)
  (Input|EnableInput (Game|GetPlayerController 0))
  (Utilities|FlowControl|Gate true) ; enters at Open
)

(event OnComponentEndOverlap(interactionbox)
  (params (OverlappedComponent :type Primitive%20Component%20Object%20Reference) (OtherActor :type Actor%20Object%20Reference) (OtherComp :type Primitive%20Component%20Object%20Reference) (OtherBodyIndex :type Integer))
  (Utilities|Casting|CastToThirdPersonCharacter OtherActor)
  (Widget|RemovefromParent (stale OnComponentBeginOverlap(interactionbox) _returnvalue)))

(event Input|ActionEvents|InputActionInteract
  (params (Key :type Key%20Structure :default "None"))
  (:Pressed
    (Variables|/Game/Blueprints/UseEtointeract.UseEtointeract_C|SetIs%20Pressed? (stale OnComponentBeginOverlap(interactionbox) _returnvalue) true)
    (Utilities|FlowControl|Delay 0.25)
    (Variables|/Game/Blueprints/UseEtointeract.UseEtointeract_C|SetIs%20Pressed? (stale OnComponentBeginOverlap(interactionbox) _returnvalue) false)
    (Utilities|FlowControl|Gate true
      (:Exit
        (|ButtonPushAnimation
          (:Finished
            (Utilities|FlowControl|FlipFlop
              (:A
                (bind _door_anim (Timeline|Door%20Timeline Play)
                  (:Update
                    (Transformation|SetRelativeRotation (Variables|Default|GetStaticMesh) (Math|Rotator|MakeRotator 0.0 0.0 (Math|Float|Lerp (Variables|Default|GetClosed%20Angle) (Variables|Default|GetOpen%20Angle) _door_anim)) false false))))
              (:B
                (Timeline|Door%20Timeline Reverse)))))))))

(fn ConstructionScript
  (Transformation|SetRelativeTransform (Variables|Default|GetButton) (Variables|Default|GetButton%20Transform) false false))