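; MoopKey is a key pickup actor that grants the ThirdPersonCharacter its HasKey4 flag.
; Box overlap shows a "use E to interact" widget, enables player input and opens a Gate, all reversed when the character leaves.
; Interact briefly flags the prompt as pressed, then, if the Gate is open, sets the flag, plays a sound, briefly shows an obtained-key widget and destroys the actor.
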(event OnComponentBeginOverlap(Box)
  (params (OverlappedComponent :type Primitive%20Component%20Object%20Reference) (OtherActor :type Actor%20Object%20Reference) (OtherComp :type Primitive%20Component%20Object%20Reference) (OtherBodyIndex :type Integer) (bFromSweep :type Boolean) (SweepResult :type Hit%20Result%20Structure%20%28by%20ref%29))
  (bind _asthird_person_character (Utilities|Casting|CastToThirdPersonCharacter OtherActor))
  (bind _returnvalue (UserInterface|CreateWidget "/Game/Blueprints/UseEtointeract.UseEtointeract_C"))
  (UserInterface|Viewport|AddtoViewport _returnvalue 0)
  (Input|EnableInput (Game|GetPlayerController 0))
  (Utilities|FlowControl|Gate true) ; enters at Open
)

(event OnComponentEndOverlap(Box)
  (params (OverlappedComponent :type Primitive%20Component%20Object%20Reference) (OtherActor :type Actor%20Object%20Reference) (OtherComp :type Primitive%20Component%20Object%20Reference) (OtherBodyIndex :type Integer))
  (Utilities|Casting|CastToThirdPersonCharacter OtherActor)
  (Widget|RemovefromParent (stale OnComponentBeginOverlap(Box) _returnvalue))
  (Input|DisableInput (Game|GetPlayerController 0))
  (Utilities|FlowControl|Gate true) ; enters at Close
)

(event Input|ActionEvents|InputActionInteract
  (params (Key :type Key%20Structure :default "None"))
  (:Pressed
    (Variables|/Game/Blueprints/UseEtointeract.UseEtointeract_C|SetIs%20Pressed? (stale OnComponentBeginOverlap(Box) _returnvalue) true)
    (Utilities|FlowControl|Delay 0.2)
    (Variables|/Game/Blueprints/UseEtointeract.UseEtointeract_C|SetIs%20Pressed? (stale OnComponentBeginOverlap(Box) _returnvalue) false)
    (Utilities|FlowControl|Gate true
      (:Exit
        (Variables|/Game/ThirdPersonBP/Blueprints/ThirdPersonCharacter.ThirdPersonCharacter_C|SetHas%20key%204? (stale OnComponentBeginOverlap(Box) _asthird_person_character) true)
        (Audio|PlaySoundatLocation "/Engine/VREditor/Sounds/UI/Camera_Shutter.Camera_Shutter" "0, 0, 0" "0, 0, 0" 1.0 1.0 0.0 0 0 0)
        (bind _returnvalue (UserInterface|CreateWidget "/Game/Blueprints/ObtainedKey.ObtainedKey_C"))
        (UserInterface|Viewport|AddtoViewport _returnvalue 0)
        (Utilities|FlowControl|Delay 1.0)
        (Widget|RemovefromParent _returnvalue)
        (Actor|DestroyActor)))))

(fn ConstructionScript)